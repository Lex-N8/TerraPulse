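; Player character for a side-scrolling platformer with jump, crouch, double jump, dash, coin pickup and healing.
; Enhanced Input drives movement along world X, flipping control yaw with acceleration direction.
; ChequeoSalto limits double jumps until landing; dash launches forward with gravity suspended until a timer restores it, then cools down.
; Retriggerable delays time coyote and double-jump window flags, though nothing here reads them; debug prints report events.
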(event Custom|EndDash
  (Variables|/Script/Engine.CharacterMovementComponent|SetGravityScale (Variables|Character|GetCharacterMovement) 2.3)
  (Utilities|Time|ClearTimerbyFunctionName 0 ""))

(event Input|EnhancedActionEvents|EnhancedInputActionIA_Agacharse
  (params (ActionValue :type Boolean) (ElapsedSeconds :type Float%20%28double-precision%29) (TriggeredSeconds :type Float%20%28double-precision%29) (InputAction :type Input%20Action%20Object%20Reference :default "/Game/Inputs/IA_Agacharse.IA_Agacharse"))
  (:Started
    (Character|Crouch))
  (:Completed
    (Character|UnCrouch)))

(event Input|EnhancedActionEvents|EnhancedInputActionIA_Movimiento
  (params (ActionValue :type Float%20%28double-precision%29) (ElapsedSeconds :type Float%20%28double-precision%29) (TriggeredSeconds :type Float%20%28double-precision%29) (InputAction :type Input%20Action%20Object%20Reference :default "/Game/Inputs/IA_Movimiento.IA_Movimiento"))
  (bind _returnvalue (Pawn|GetController))
  (Pawn|Input|AddMovementInput "1.000000,0.000000,0.000000" ActionValue false)
  (Math|Float|CompareFloat (.x (Pawn|Components|CharacterMovement|GetCurrentAcceleration (Variables|Character|GetCharacterMovement))) 0.0
    (:>
      (Pawn|SetControlRotation _returnvalue (Math|Rotator|MakeRotator 0.0 0.0 0.0)))
    (:<
      (Pawn|SetControlRotation _returnvalue (Math|Rotator|MakeRotator 0.0 0.0 1.8e+02)))))

(event Input|EnhancedActionEvents|EnhancedInputActionIA_Jump
  (params (ActionValue :type Boolean) (ElapsedSeconds :type Float%20%28double-precision%29) (TriggeredSeconds :type Float%20%28double-precision%29) (InputAction :type Input%20Action%20Object%20Reference :default "/Game/Inputs/IA_Jump.IA_Jump"))
  (:Started
    (Character|Jump))
  (:Completed
    (Character|StopJumping)))

(event Input|EnhancedActionEvents|EnhancedInputActionIA_DobleSalto
  (params (ActionValue :type Boolean) (ElapsedSeconds :type Float%20%28double-precision%29) (TriggeredSeconds :type Float%20%28double-precision%29) (InputAction :type Input%20Action%20Object%20Reference :default "/Game/Inputs/IA_DobleSalto.IA_DobleSalto"))
  (:Started
    (if (Variables|Default|GetPuede%20Saltar?)
      (CallFunction|ChequeoSalto)
      (Character|Jump)))
  (:Completed
    (Character|StopJumping)))

(event Input|EnhancedActionEvents|EnhancedInputActionIA_Dash
  (params (ActionValue :type Boolean) (ElapsedSeconds :type Float%20%28double-precision%29) (TriggeredSeconds :type Float%20%28double-precision%29) (InputAction :type Input%20Action%20Object%20Reference :default "/Game/Inputs/IA_Dash.IA_Dash"))
  (:Started
    (if (Variables|Default|GetPuedo%20Hacer%20Dash?)
      (Variables|Default|SetPuedo%20Hacer%20Dash? false)
      (Variables|/Script/Engine.CharacterMovementComponent|SetGravityScale (Variables|Character|GetCharacterMovement) 0.0)
      (Character|LaunchCharacter (* (Transformation|GetActorForwardVector) (Variables|Default|GetVelocidadDash)) false false)
      (Utilities|Time|SetTimerbyEvent (delegate Custom|EndDash) (Variables|Default|GetTiempodeDash))
      (Utilities|FlowControl|Delay (Variables|Default|GetTiempo%20para%20volver%20a%20hacer%20un%20dash))
      (Variables|Default|SetPuedo%20Hacer%20Dash? true))))

(event EventBeginPlay
  (bind _asplayer_controller (Utilities|Casting|CastToPlayerController (Pawn|GetController)))
  (Input|AddMappingContext (PlayerController|LocalPlayerSubsystems|GetEnhancedInputLocalPlayerSubsystem _asplayer_controller) "/Game/Inputs/Mapping/IMC_RH.IMC_RH" 0 "(bIgnoreAllPressedKeysUntilRelease=True,bForceImmediately=False,bNotifyUserSettings=False)"))

(event EventObtenerMonedas
  (params (Monedas :type Integer))
  (bind _output_get (Variables|Default|SetMonedas (+ Monedas (Variables|Default|GetMonedas))))
  (Development|PrintString (Utilities|String|Append "Agarraste 1 moneda, tus monedas actuales son:  
 
" (Utilities|String|ToString(Integer) _output_get)) true true "(R=0.000000,G=0.660000,B=1.000000,A=1.000000)" 5.0))

(event EventCurar
  (params (RegenSalud :type Float%20%28double-precision%29))
  (bind _output_get (Variables|Default|SetVida (+ RegenSalud (Variables|Default|GetVida))))
  (Development|PrintString (Utilities|String|Append "Tu heroe se esta curando: 
" (Utilities|String|ToString(Float) _output_get)) true true "(R=0.000000,G=0.660000,B=1.000000,A=1.000000)" 1.0 "Salud"))

(event EventOnLanded
  (params (Hit :type Hit%20Result%20Structure%20%28by%20ref%29))
  (Development|PrintString "Hello")
  (Variables|Default|SetPrimer%20Salto%20Hecho false)
  (Variables|Default|SetPuede%20Saltar? true))

(event EventOnJumped
  (Development|PrintString "salto")
  (Variables|Default|SetDisponible%20doble%20salto true)
  (Utilities|FlowControl|RetriggerableDelay (Variables|Default|GetTiempo%20para%20Doble%20Salto))
  (Variables|Default|SetDisponible%20doble%20salto false))

(event EventOnWalkingOffLedge
  (params (PreviousFloorImpactNormal :type Vector%20%28by%20ref%29 :default "0, 0, 0") (PreviousFloorContactNormal :type Vector%20%28by%20ref%29 :default "0, 0, 0") (PreviousLocation :type Vector%20%28by%20ref%29 :default "0, 0, 0") (TimeDelta :type Float%20%28single-precision%29))
  (Development|PrintString "sali del suelo")
  (Variables|Default|SetEsta%20en%20tiempo%20de%20coyote? true)
  (Utilities|FlowControl|RetriggerableDelay (Variables|Default|GetTiempo%20de%20Coyote))
  (Variables|Default|SetEsta%20en%20tiempo%20de%20coyote? false))

(fn ConstructionScript)

(fn ChequeoSalto
  (if (Variables|Default|GetPrimer%20Salto%20Hecho)
    (Variables|Default|SetPrimer%20Salto%20Hecho false)
    (Variables|Default|SetPuede%20Saltar? false)
    (else
      (Variables|Default|SetPrimer%20Salto%20Hecho true))))